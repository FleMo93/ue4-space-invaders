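; BP_ProtectionWall is a damageable wall actor that shows hit feedback and is removed when killed.
; BeginPlay hands a dynamic damage-indicator material to BCDamageIndicator, which BC_Damagable's damage event triggers.
; On kill, the server destroys the actor, while clients only print a debug string.
; Procedural mesh slicing nodes, with helpers computing evenly spaced box cut positions, are unconnected and never run.
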(event Damage(BC_Damagable)
  (params (Damage :type Float%20%28single-precision%29))
  (CallFunction|OnDamage))

(event Killed(BC_Damagable)
  (CallFunction|OnKill))

(event EventBeginPlay
  (bind _returnvalue (Rendering|Material|CreateDynamicMaterialInstance (Variables|Default|GetProtectionWallMesh) 0 "/Game/Materials/M_Damage_Indicator_Wall.M_Damage_Indicator_Wall" "None" :!class /Script/Engine.PrimitiveComponent))
  (Default|AddMaterialInstance (Variables|Default|GetBC_DamageIndicator) _returnvalue))

(fn ConstructionScript)

(fn GetBoxSlicingPositions
  (params (Box :type Box%20Component%20Object%20Reference) (ColumnSlices :type Integer) (RowSlices :type Integer) (RefColumns :type Array%20of%20Vectors) (RefRows :type Array%20of%20Vectors))
  (bind _boxextent (Variables|/Script/Engine.BoxComponent|GetBoxExtent Box))
  (bind (_x _y _z) (Math|Vector|BreakVector _boxextent))
  (bind _returnvalue (* _x -1.0))
  (bind _returnvalue_2 (* _z -1.0))
  (Utilities|FlowControl|Sequence
    (:then_0
      (bind _outpuarraytofill (CallFunction|GetEvenPositionsfromRange (Math|Float|Min(Float) _returnvalue _x) (Math|Float|Max(Float) _returnvalue _x) ColumnSlices (Utilities|Array|MakeArray)))
      (for _array_element _outpuarraytofill
        (Utilities|Array|Add RefColumns (Math|Vector|MakeVector _array_element 0.0 0.0))))
    (:then_1
      (bind _outpuarraytofill_2 (CallFunction|GetEvenPositionsfromRange (Math|Float|Min(Float) _z _returnvalue_2) (Math|Float|Max(Float) _z _returnvalue_2) RowSlices (Utilities|Array|MakeArray)))
      (for _array_element_2 _outpuarraytofill_2
        (Utilities|Array|Add RefRows (Math|Vector|MakeVector 0.0 0.0 _array_element_2))))
    (:then_2
      (return RefColumns RefRows))))

(fn GetEvenPositionsfromRange
  (params (From :type Float%20%28single-precision%29) (To :type Float%20%28single-precision%29) (NumberOfPositions :type Integer) (ArrayToFill :type Array%20of%20Floats%20%28single-precision%29))
  (bind _returnvalue (Math|Float|Min(Float) From To))
  (for _index (range 1 NumberOfPositions)
    (Utilities|Array|Add ArrayToFill (+ (* _index (/ (- (Math|Float|Max(Float) From To) _returnvalue) (Math|Conversions|ToFloat(Integer) (+ NumberOfPositions 1)))) _returnvalue)))
  (return ArrayToFill))

(fn OnDamage
  (Default|Damage (Variables|Default|GetBC_DamageIndicator)))

(fn OnKill
  (if (Networking|IsServer)
    (Actor|DestroyActor)
    (else
      (Development|PrintString "Client kill"))))