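; Player controller for a networked spaceship game that manages the player's ship, level camera and debug HUD.
; On BeginPlay, controller ID 0 switches view to the level camera and creates a debug widget showing server status, with ping refreshed on Tick.
; SpawnPawn, on authority only, spawns and possesses a ship if the player is dead and binds its damageable component's Killed event.
; PawnKilled clears the alive flag and fires OnPlayerKilled.
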(event Custom|Pawn%20Killed
  (Variables|Default|SetIs%20Alive false)
  (Default|CallOnPlayerKilled))

(event EventBeginPlay
  (CallFunction|SetCamera)
  (CallFunction|SpawnHUD))

(event EventTick
  (params (DeltaSeconds :type Float%20%28single-precision%29))
  (CallFunction|UpdateHUD))

(fn ConstructionScript)

(fn SpawnPawn
  (Networking|SwitchHasAuthority
    (:Authority
      (if (not (Variables|Default|GetIs%20Alive))
        (Variables|Default|SetIs%20Alive true)
        (Actor|GetActorOfClass "/Game/Game.Game_C")
        (bind _returnvalue (Game|SpawnActorfromClass "/Game/BP_PlayerSpaceShip.BP_PlayerSpaceShip_C" (Math|Transform|MakeTransform "0, 0, 0") "AlwaysSpawn" 0 0))
        (Pawn|Possess _returnvalue)
        (EventDispatchers|BindEventtoKilled (Actor|GetComponentbyClass _returnvalue "/Game/BC_Damagable.BC_Damagable_C") (EventDispatchers|CreateEvent :!event Custom|Pawn%20Killed))
        (return _returnvalue)))))

(fn SpawnHUD
  (if (== (Class|GameplayStatics|GetPlayerControllerID self) 0)
    (bind _returnvalue (UserInterface|CreateWidget "/Game/HUD/DebugInfo.DebugInfo_C"))
    (UserInterface|Viewport|AddtoViewport _returnvalue 0)
    (Variables|Default|SetHUD%20Debug%20Info _returnvalue)
    (Networking|SwitchHasAuthority
      (:Authority
        (Rendering|Components|TextRender|SetText (Variables|/Game/HUD/DebugInfo.DebugInfo_C|GetIsServer _returnvalue) "true"))
      (:Remote
        (Rendering|Components|TextRender|SetText (Variables|/Game/HUD/DebugInfo.DebugInfo_C|GetIsServer _returnvalue) "false")))))

(fn SetCamera
  (if (== (Class|GameplayStatics|GetPlayerControllerID self) 0)
    (bind _returnvalue (Actor|GetActorOfClass "/Game/C_LevelCam.C_LevelCam_C"))
    (Game|Player|SetViewTargetwithBlend _returnvalue 0.0 "VTBlend_Linear" 0.0 false)))

(fn UpdateHUD
  (bind _hud_debug_info (Variables|Default|GetHUD%20Debug%20Info))
  (bind _playerstate (Variables|GetPlayerState))
  (if (!= _playerstate 0)
    (if (!= _hud_debug_info 0)
      (Rendering|Components|TextRender|SetText (Variables|/Game/HUD/DebugInfo.DebugInfo_C|GetPing _hud_debug_info) (Utilities|Text|ToText(String) (Variables|/Script/Engine.PlayerState|GetPing _playerstate))))))