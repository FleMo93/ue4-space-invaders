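; BP_Bullet is a projectile actor that deals damage to what it overlaps and then disappears.
; On BeginPlay it drives its ProjectileMovement at Speed along the local Z axis, and Tick destroys it once its lifetime exceeds DestroyAfter.
; Overlapping any actor other than its owner destroys it and, guarded by a one-shot CanDamage flag, sends DamageEvent to that actor's BC_Damagable component.
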(event EventBeginPlay
  (bind _projectilemovement (Variables|Default|GetProjectileMovement))
  (bind _speed (Variables|Default|GetSpeed))
  ;[1 1 1] Initialize movement
  (Variables|/Script/Engine.ProjectileMovementComponent|SetMaxSpeed _projectilemovement _speed)
  (Variables|/Script/Engine.ProjectileMovementComponent|SetInitialSpeed _projectilemovement _speed)
  (Game|Components|ProjectileMovement|SetVelocityinLocalSpace _projectilemovement (Math|Vector|MakeVector 0.0 0.0 _speed)))

(event Collision|EventActorBeginOverlap
  (params (OtherActor :type Actor%20Object%20Reference))
  (bind _returnvalue (Actor|GetComponentbyClass OtherActor "/Game/BC_Damagable.BC_Damagable_C"))
  (if (not (== OtherActor (Components|GetOwner)))
    (Actor|DestroyActor)
    (if (Variables|Default|GetCanDamage)
      (Variables|Default|SetCanDamage false)
      (if (Utilities|IsValid OtherActor)
        (if (Utilities|IsValid _returnvalue)
          (Default|DamageEvent _returnvalue 1.0))))))

(event EventTick
  (params (DeltaSeconds :type Float%20%28single-precision%29))
  ;[1 1 1] Destroy after time
  (if (>= (Actor|GetGameTimeSinceCreation) (Variables|Default|GetDestroy%20After))
    (Actor|DestroyActor)))

(fn ConstructionScript)