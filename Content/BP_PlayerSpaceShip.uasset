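; BP_PlayerSpaceShip is the player-controlled spaceship, which moves horizontally and shoots.
; Input events forward the horizontal axis to MoveByAxis and the Shoot press to the BCShootable component.
; Its construction script copies left and right area bounds from the BP_PlayArea actor found in the world.
; On BeginPlay, a locally controlled ship swaps its mesh material, setting it apart visually.
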(event EventBeginPlay
  (if (Pawn|IsLocallyControlled)
    (Rendering|Material|SetMaterial (Variables|Default|GetSpaceShipMesh) 0 "/Engine/MapTemplates/Materials/BasicAsset01.BasicAsset01")))

(event Input|ActionEvents|InputActionShoot
  (params (Key :type Key%20Structure :default "None"))
  (:Pressed
    (Default|Shoot (Variables|Default|GetBC_Shootable))))

(event Input|AxisEvents|InputAxisMoveHorizontal
  (params (AxisValue :type Float%20%28single-precision%29))
  (Class|MyPlayerCharacter|MovebyAxis AxisValue))

(fn ConstructionScript
  (bind _returnvalue (Actor|GetActorOfClass "/Game/BP_PlayArea.BP_PlayArea_C"))
  (Variables|Default|SetLeftAreaBound (Variables|/Game/BP_PlayArea.BP_PlayArea_C|GetLeft _returnvalue))
  (Variables|Default|SetRightAreaBound (Variables|/Game/BP_PlayArea.BP_PlayArea_C|GetRight _returnvalue)))