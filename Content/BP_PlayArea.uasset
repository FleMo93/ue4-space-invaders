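; BP_PlayArea is an actor that defines a rectangular play area on the X-Z plane from its Box component.
; The construction script adds and subtracts the box extent from the bounds origin to store Left, Right, Top and Bottom edge values.
; Y is ignored, and the event graph has no runtime logic.
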(event EventBeginPlay)

(event Collision|EventActorBeginOverlap
  (params (OtherActor :type Actor%20Object%20Reference)))

(event EventTick
  (params (DeltaSeconds :type Float%20%28single-precision%29)))

(fn ConstructionScript
  (bind _box (Variables|Default|GetBox))
  (bind (_origin _boxextent) (Collision|GetComponentBounds _box))
  (bind (_x _y _z) (Math|Vector|BreakVector _origin))
  (bind (_x_2 _y_2 _z_2) (Math|Vector|BreakVector _boxextent))
  (Variables|Default|SetRight (+ _x _x_2))
  (Variables|Default|SetTop (+ _z _z_2))
  (Variables|Default|SetLeft (- _x _x_2))
  (Variables|Default|SetBottom (- _z _z_2)))