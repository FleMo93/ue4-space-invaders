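; BP_Enemy is a server-authoritative enemy actor that harms damageable actors on contact.
; On BeginPlay, the authority binds its BC_Damagable component's killed callback to destroy the actor.
; On overlap, the server finds a BC_Damagable component on the other actor and applies a fixed, heavy damage hit through it.
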(event Custom|Killed%20Event
  (Actor|DestroyActor))

(event EventBeginPlay
  (Networking|SwitchHasAuthority
    (:Authority
      (EventDispatchers|AssignKilled (Variables|Default|GetBC_Damagable) (delegate Custom|Killed%20Event)))))

(event Collision|EventActorBeginOverlap
  (params (OtherActor :type Actor%20Object%20Reference))
  (bind _returnvalue (Actor|GetComponentbyClass OtherActor "/Game/BC_Damagable.BC_Damagable_C"))
  (if (Networking|IsServer)
    (if (Utilities|IsValid _returnvalue)
      (Default|DamageEvent _returnvalue 1e+02))))

(fn ConstructionScript)