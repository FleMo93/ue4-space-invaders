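; BP_MyEnemyBlock is a grid formation of BP_Enemy actors that periodically fires at random.
; Its construction script copies side bounds from BP_PlayArea and places the block at the top-left.
; On BeginPlay, only the authority spawns the rows and columns and starts a looping shoot timer.
; Shoot picks from random EnemyColumns, targeting a last-in-column enemy, and fires through its BC_Shootable component.
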(event Custom|Event%20Shoot
  (bind _enemycolumns (Variables|Default|GetEnemyColumns))
  (bind _outitem (Utilities|Array|Random _enemycolumns))
  (bind _enemies (Utilities|Struct|BreakEnemyColumn _outitem))
  (bind _asbp_enemy (Utilities|Casting|CastToBP_Enemy (Utilities|Array|Get(acopy) _enemies (Utilities|Array|LastIndex _enemies))))
  (if (Utilities|IsValid (Actor|GetComponentbyClass _asbp_enemy "/Game/BC_Shootable.BC_Shootable_C"))
    (Default|Shoot (Actor|GetComponentbyClass _asbp_enemy "/Game/BC_Shootable.BC_Shootable_C"))))

(event EventBeginPlay
  (Networking|SwitchHasAuthority
    (:Authority
      (Class|EnemyBlock|SpawnEnemies (Variables|Default|GetColumns) (Variables|Default|GetRows) (Variables|Default|GetSpawnOffset) "/Game/BP_Enemy.BP_Enemy_C")
      (Utilities|Time|SetTimerbyEvent (delegate Custom|Event%20Shoot) (Variables|Default|GetShooting%20Intervall) true))))

(fn ConstructionScript
  (bind _returnvalue (Actor|GetActorOfClass "/Game/BP_PlayArea.BP_PlayArea_C"))
  (bind _output_get (Variables|Default|SetLeftBound (Variables|/Game/BP_PlayArea.BP_PlayArea_C|GetLeft _returnvalue)))
  (Variables|Default|SetRightBound (Variables|/Game/BP_PlayArea.BP_PlayArea_C|GetRight _returnvalue))
  (Transformation|SetActorLocation (Math|Vector|MakeVector _output_get 0.0 (Variables|/Game/BP_PlayArea.BP_PlayArea_C|GetTop _returnvalue)) false false))